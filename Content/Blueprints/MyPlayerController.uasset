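; Player controller that drives both a human pawn and an alien from one set of inputs.
; On BeginPlay it spawns an Alien and a MyPlayerController2 to possess it, yet handles alien input itself through the stored reference.
; Separate axis mappings move each character along world X and Y.
; The alien's ability1 action fires a Projectile1 along its facing, and the X key spawns an Aoe forcefield attached to it.
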(event EventBeginPlay
  (bind _returnvalue (Math|Transform|MakeTransform "140.000000, 0,225.000000" "0.000000,90.000000,0.000000"))
  ;[1 1 1] Spawn Alien
  (bind _returnvalue_2 (Game|SpawnActorfromClass "/Game/Blueprints/MyPlayerController2.MyPlayerController2_C" _returnvalue "Undefined" 0 0))
  (Variables|Default|Setcontroller2 _returnvalue_2)
  (bind _returnvalue_3 (Game|SpawnActorfromClass "/Game/Blueprints/Blueprints/characters/alien.alien_C" _returnvalue "Undefined" 0 0))
  (Variables|Default|Setalien _returnvalue_3)
  (Pawn|Possess (Variables|Default|Getcontroller2) (Variables|Default|Getalien)))

(event Input|ActionEvents|InputActionability1
  (params (Key :type Key%20Structure))
  (bind _alien (Variables|Default|Getalien))
  (bind _returnvalue (Transformation|GetActorRotation _alien))
  ;[1 1 1] Alien Controls
  ;;[1 1 1] Ability 1 (Fire straight Using Z)
  (:Pressed
    (Game|SpawnActorfromClass "/Game/Blueprints/Blueprints/projectiles/projectile1.projectile1_C" (Math|Transform|MakeTransform (+ (Transformation|GetActorLocation _alien) (* (Math|Vector|GetForwardVector _returnvalue) 1e+02)) _returnvalue) "Undefined" 0 0)))

(event Input|AxisEvents|InputAxisalienX
  (params (AxisValue :type Float%20%28single-precision%29))
  ;[1 1 1] Alien Controls
  ;;[1 1 1] Movement
  (Pawn|Input|AddMovementInput (Variables|Default|Getalien) "1.000000, 0, 0" AxisValue false))

(event Input|AxisEvents|InputAxisalienY
  (params (AxisValue :type Float%20%28single-precision%29))
  ;[1 1 1] Alien Controls
  ;;[1 1 1] Movement
  (Pawn|Input|AddMovementInput (Variables|Default|Getalien) "0,1.000000, 0" AxisValue false))

(event Input|AxisEvents|InputAxishumanX
  (params (AxisValue :type Float%20%28single-precision%29))
  ;[1 1 1] Human Controls
  (Pawn|Input|AddMovementInput (Pawn|GetControlledPawn) "1.000000, 0, 0" AxisValue false))

(event Input|AxisEvents|InputAxishumanY
  (params (AxisValue :type Float%20%28single-precision%29))
  ;[1 1 1] Human Controls
  (Pawn|Input|AddMovementInput (Pawn|GetControlledPawn) "0,1.000000, 0" AxisValue false))

(event Input|KeyboardEvents|X
  (params (Key :type Key%20Structure))
  (bind _alien (Variables|Default|Getalien))
  ;[1 1 1] Alien Controls
  ;;[1 1 1] AoE Ability (forcefield w/ X key)
  (:Pressed
    (bind _returnvalue (Game|SpawnActorfromClass "/Game/Blueprints/Blueprints/projectiles/aoe.aoe_C" (Math|Transform|MakeTransform (Transformation|GetActorLocation _alien) "0, 0, 0" "2.500000,2.500000,2.500000") "Undefined" 0 0))
    (Transformation|AttachActorToActor _returnvalue _alien "None" "SnapToTarget" "KeepRelative" "KeepRelative" true)))

(event Input|KeyboardEvents|C
  (params (Key :type Key%20Structure))
  ;[1 1 1] Alien Controls
)

(fn ConstructionScript)